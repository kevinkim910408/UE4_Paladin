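; Goblin melee enemy that chases and slashes the player, measuring distance and direction along the Y axis only.
; Tick drives an idle, follow and attack state machine by distance, idling when the player dies.
; Animation-timed events toggle the sword capsule, whose overlap applies damage, and repeat the slash or resume the chase.
; Taking damage briefly swaps the material; zero HP plays a death montage, disables collision and destroys the actor after a delay.
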(event `self.ReceiveTick`
  (params (DeltaSeconds :type "Float (single-precision)"))
  ;[1 1 1] Movement Animation
  (`self.SaveDistance/Dir`)
  (if (`self.IsPlayerDeath`)
    (set `self.CurState` "NewEnumerator3"))
  (switch `/Game/Enums/MonsterState` (`self.CurState`)
    (:`NewEnumerator0`
      (if (<= (`self.DistanceBtwPlayer`) 800.0)
        (set `self.CurState` "NewEnumerator1")))
    (:`NewEnumerator1`
      (if (<= (`self.DistanceBtwPlayer`) 160.0)
        (set `self.CurState` "NewEnumerator2")
        (`self.PlayAnimMontage` "/Game/Mesh/Monster/Animation/sword_and_shield_slash_Montage.sword_and_shield_slash_Montage")
        (set `self.IsAttacking` true)
        (else
          (`self.AddMovementInput` (`self.DirtoPlayer`)))))
    (:`NewEnumerator2`
      (if (`self.IsAttacking`)
        _
        (elif (>= (`self.DistanceBtwPlayer`) 180.0)
          (set `self.CurState` "NewEnumerator1"))))))

(event `self.ReceiveAnyDamage`
  (params (Damage :type "Float (single-precision)") (DamageType :type "DamageType Object Reference") (InstigatedBy :type "Controller Object Reference") (DamageCauser :type "Actor Object Reference"))
  ;[1 1 1] Get Damage
  (bind _output_get (set `self.HP` (- (`self.HP`) Damage)))
  (`self.ChangeDamageColor`)
  (if (<= _output_get 0.0)
    (`self.PlayAnimMontage` "/Game/Mesh/Monster/Animation/sword_and_shield_death_Montage.sword_and_shield_death_Montage")
    (set `self.CurState` "NewEnumerator4")
    (`PrimitiveComponent.SetCollisionEnabled` (`self.CapsuleComponent`) "NoCollision")
    (`PrimitiveComponent.SetCollisionEnabled` (`self.Capsule`) "NoCollision")
    (`KismetSystemLibrary.Delay` 3.0)
    (`self.K2_DestroyActor` self)))

(event `OnAnimEnd_Attack`
  ;[1 1 1] After Attack, Check distance - follow or attack
  (set `self.IsAttacking` false)
  (if (`self.IsPlayerDeath`)
    (set `self.CurState` "NewEnumerator3")
    (else
      (`self.K2_SetActorRotation` (`KismetMathLibrary.Conv_VectorToRotator` (`self.DirtoPlayer`)))
      (if (>= (`self.DistanceBtwPlayer`) 180.0)
        (set `self.CurState` "NewEnumerator1")
        (else
          (`self.PlayAnimMontage` "/Game/Mesh/Monster/Animation/sword_and_shield_slash_Montage.sword_and_shield_slash_Montage")
          (set `self.IsAttacking` true))))))

(event `ChangeDamageColor`
  (bind _mesh (`self.Mesh`))
  ;[1 1 1] ChangeDamageColor
  (`PrimitiveComponent.SetMaterial` _mesh 0 "/Game/Mesh/Monster/phong1_Inst.phong1_Inst")
  (`KismetSystemLibrary.Delay` 0.2)
  (`PrimitiveComponent.SetMaterial` _mesh 0 "/Game/Mesh/Monster/phong1.phong1"))

(event `SaveDistance/Dir`
  (bind _returnvalue (`GameplayStatics.GetPlayerCharacter` 0))
  (bind _returnvalue_2 (`KismetMathLibrary.MakeVector` 0.0 (.y (- (`self.K2_GetActorLocation` _returnvalue) (`self.K2_GetActorLocation`)))))
  ;[1 1 1] Save Distance and Dir btw Player and Goblin
  (bind _asbp_character (cast `/Game/BP/BP_Character` _returnvalue))
  (set `self.IsPlayerDeath` (`/Game/BP/BP_Character.IsDeath` _asbp_character))
  (set `self.DistanceBtwPlayer` (`KismetMathLibrary.VSize` _returnvalue_2))
  (set `self.DirtoPlayer` (`KismetMathLibrary.Normal` _returnvalue_2)))

(event `self.Capsule.OnComponentBeginOverlap`
  (params (OverlappedComponent :type "PrimitiveComponent Object Reference") (OtherActor :type "Actor Object Reference") (OtherComp :type "PrimitiveComponent Object Reference") (OtherBodyIndex :type Integer) (bFromSweep :type Boolean) (SweepResult :type "HitResult Structure (by ref)"))
  ;[1 1 1] Damage to Player
  (if (!= OtherActor self)
    (if (!= (`|GetArrayItem` (`Actor.Tags` OtherActor)) (`|GetArrayItem` (`self.Tags`)))
      (if (== (`|GetArrayItem` (`ActorComponent.ComponentTags` OtherComp)) "character")
        (`GameplayStatics.ApplyDamage` OtherActor (`self.Atk`) null self)))))

(event `OnColStart_Attack`
  ;[1 1 1] Collision of Sword Capsule
  (`PrimitiveComponent.SetCollisionEnabled` (`self.Capsule`) "QueryAndPhysics"))

(event `OnColEnd_Attack`
  ;[1 1 1] Collision of Sword Capsule
  (`PrimitiveComponent.SetCollisionEnabled` (`self.Capsule`) "NoCollision"))

(fn `UserConstructionScript`)