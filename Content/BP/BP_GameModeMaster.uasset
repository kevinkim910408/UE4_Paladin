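; Game mode Blueprint that ends the stage with a clear screen when the boss reaches a specific state.
; On BeginPlay it caches the first actor tagged "Boss" as a BP_Boss reference.
; Tick polls that boss's CurState and, on the target enum value, adds the WBP_StageClear widget to the viewport, shows the mouse cursor and pauses the game.
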(event `self.ReceiveBeginPlay`
  ;[1 1 1] Boss 변수만든거에 Boss 정보 넣어주기
  (bind _outactors (`GameplayStatics.GetAllActorsWithTag` "Boss"))
  (bind _asbp_boss (cast `/Game/BP/BP_Boss` (`|GetArrayItem` _outactors)))
  (set `self.Boss` _asbp_boss))

(event `self.ReceiveTick`
  (params (DeltaSeconds :type "Float (single-precision)"))
  (bind _returnvalue (`GameplayStatics.GetPlayerController` 0))
  (if (`|EnumEquality` (`/Game/BP/BP_Boss.CurState` (`self.Boss`)) "NewEnumerator4")
    (bind _returnvalue_2 (`|CreateWidget` "/Game/BP/WBP/WBP_StageClear.WBP_StageClear_C" _returnvalue))
    (`UserWidget.AddToViewport` _returnvalue_2 0)
    (set `PlayerController.bShowMouseCursor` true _returnvalue)
    (`GameplayStatics.SetGamePaused` true)))

(fn `UserConstructionScript`)