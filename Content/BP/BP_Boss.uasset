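; Boss enemy that chases and melees the player along the Y axis.
; A Tick-driven state machine follows the player and starts attacks, swapping a punch for a telegraphed skill swipe when a recursive Delay timer has charged.
; Attack events toggle two weapon capsules whose tag-filtered overlaps apply normal or skill damage, and the attack-end event chooses to repeat or follow.
; Incoming damage flashes the material, and zero HP triggers death and delayed destruction.
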(event `StartAttack`
  ;[1 1 1] StartAttack - custom Event
  (set `self.IsAttacking` true)
  (if (>= (`self.SkillTime`) 8.0)
    (set `self.CurState` "NewEnumerator5")
    (`self.K2_SetActorRotation` (`KismetMathLibrary.Conv_VectorToRotator` (`self.DirtoPlayer`)))
    (`PrimitiveComponent.SetMaterial` (`self.Mesh`) 0 "/Game/Mesh/Boss1/Ch44_body1_Inst1.Ch44_body1_Inst1")
    (set `self.SkillTime` 0.0)
    (`self.PlayAnimMontage` "/Game/Mesh/Boss1/Animation/mutant_flexing_muscles_Montage.mutant_flexing_muscles_Montage" 1.0 "Start")
    (`KismetSystemLibrary.Delay` 2.0)
    (`self.PlayAnimMontage` "/Game/Mesh/Boss1/Animation/mutant_swiping_Montage.mutant_swiping_Montage")
    (`GameplayStatics.PlaySound2D` "/Game/Sound/Que/SwingSword.SwingSword" 1.0 1.0 0.0 null null)
    (else
      (set `self.CurState` "NewEnumerator2")
      (`self.PlayAnimMontage` "/Game/Mesh/Boss1/Animation/mutant_punch_Montage.mutant_punch_Montage")
      (`GameplayStatics.PlaySound2D` "/Game/Sound/Que/SwingSword.SwingSword" 1.0 1.0 0.0 null null))))

(event `self.ReceiveTick`
  (params (DeltaSeconds :type "Float (single-precision)"))
  ;[1 1 1] Movement Animation
  (`self.SaveDistance/Dir`)
  (if (`self.IsPlayerDeath`)
    (set `self.CurState` "NewEnumerator3"))
  (switch `/Game/Enums/MonsterState` (`self.CurState`)
    (:`NewEnumerator0`
      (if (<= (`self.DistanceBtwPlayer`) 500.0)
        (set `self.CurState` "NewEnumerator1")
        (`self.SkillTimeLoop`)))
    (:`NewEnumerator1`
      (if (<= (`self.DistanceBtwPlayer`) 130.0)
        (`self.StartAttack`)
        (else
          (`self.AddMovementInput` (`self.DirtoPlayer`)))))
    (:`NewEnumerator2`
      (if (`self.IsAttacking`)
        _
        (elif (>= (`self.DistanceBtwPlayer`) 150.0)
          (set `self.CurState` "NewEnumerator1"))))))

(event `SkillTimeLoop`
  ;[1 1 1] SkillTime Loop
  (`KismetSystemLibrary.Delay` 1.0)
  (set `self.SkillTime` (+ (`self.SkillTime`) 1.0))
  (`self.SkillTimeLoop`))

(event `self.ReceiveAnyDamage`
  (params (Damage :type "Float (single-precision)") (DamageType :type "DamageType Object Reference") (InstigatedBy :type "Controller Object Reference") (DamageCauser :type "Actor Object Reference"))
  ;[1 1 1] Get Damage
  (bind _output_get (set `self.HP` (- (`self.HP`) Damage)))
  (`self.ChangeDamageColor`)
  (if (<= _output_get 0.0)
    (`self.PlayAnimMontage` "/Game/Mesh/Boss1/Animation/mutant_dying_Montage.mutant_dying_Montage")
    (set `self.CurState` "NewEnumerator4")
    (`PrimitiveComponent.SetCollisionEnabled` (`self.CapsuleComponent`) "NoCollision")
    (`PrimitiveComponent.SetCollisionEnabled` (`self.Capsule`) "NoCollision")
    (`KismetSystemLibrary.Delay` 5.0)
    (`self.K2_DestroyActor` self)))

(event `OnAnimEnd_Attack`
  ;[1 1 1] After Attack, Check distance - follow or attack
  (`PrimitiveComponent.SetMaterial` (`self.Mesh`) 0 "/Game/Mesh/Boss1/Ch44_body1.Ch44_body1")
  (set `self.IsAttacking` false)
  (if (`self.IsPlayerDeath`)
    (set `self.CurState` "NewEnumerator3")
    (elif (>= (`self.DistanceBtwPlayer`) 180.0)
      (set `self.CurState` "NewEnumerator1")
      (else
        (`self.StartAttack`)))))

(event `ChangeDamageColor`
  (bind _mesh (`self.Mesh`))
  ;[1 1 1] ChangeDamageColor
  (`PrimitiveComponent.SetMaterial` _mesh 0 "/Game/Mesh/Boss1/Ch44_body1_Inst.Ch44_body1_Inst")
  (`KismetSystemLibrary.Delay` 0.2)
  (`PrimitiveComponent.SetMaterial` _mesh 0 "/Game/Mesh/Boss1/Ch44_body1.Ch44_body1"))

(event `SaveDistance/Dir`
  (bind _returnvalue (`GameplayStatics.GetPlayerCharacter` 0))
  (bind _returnvalue_2 (`KismetMathLibrary.MakeVector` 0.0 (.y (- (`self.K2_GetActorLocation` _returnvalue) (`self.K2_GetActorLocation`)))))
  ;[1 1 1] Save Distance and Dir btw Player and Goblin
  (bind _asbp_character (cast `/Game/BP/BP_Character` _returnvalue))
  (set `self.IsPlayerDeath` (`/Game/BP/BP_Character.IsDeath` _asbp_character))
  (set `self.DistanceBtwPlayer` (`KismetMathLibrary.VSize` _returnvalue_2))
  (set `self.DirtoPlayer` (`KismetMathLibrary.Normal` _returnvalue_2)))

(event `self.Capsule.OnComponentBeginOverlap`
  (params (OverlappedComponent :type "PrimitiveComponent Object Reference") (OtherActor :type "Actor Object Reference") (OtherComp :type "PrimitiveComponent Object Reference") (OtherBodyIndex :type Integer) (bFromSweep :type Boolean) (SweepResult :type "HitResult Structure (by ref)"))
  ;[1 1 1] Damage to Player - Normal Attack
  (if (!= OtherActor self)
    (if (!= (`|GetArrayItem` (`Actor.Tags` OtherActor)) (`|GetArrayItem` (`self.Tags`)))
      (if (== (`|GetArrayItem` (`ActorComponent.ComponentTags` OtherComp)) "character")
        (`GameplayStatics.ApplyDamage` OtherActor (`self.Atk`) null self)))))

(event `self.Capsule1.OnComponentBeginOverlap`
  (params (OverlappedComponent :type "PrimitiveComponent Object Reference") (OtherActor :type "Actor Object Reference") (OtherComp :type "PrimitiveComponent Object Reference") (OtherBodyIndex :type Integer) (bFromSweep :type Boolean) (SweepResult :type "HitResult Structure (by ref)"))
  ;[1 1 1] Damage to Player - Skill Attack
  (if (!= OtherActor self)
    (if (!= (`|GetArrayItem` (`Actor.Tags` OtherActor)) (`|GetArrayItem` (`self.Tags`)))
      (if (== (`|GetArrayItem` (`ActorComponent.ComponentTags` OtherComp)) "character")
        (`GameplayStatics.ApplyDamage` OtherActor (`self.Atk-Skill1`) null self)))))

(event `OnColStart_Attack`
  ;[1 1 1] Collision of Sword Capsule  - Normal Attack
  (`PrimitiveComponent.SetCollisionEnabled` (`self.Capsule`) "QueryAndPhysics"))

(event `OnColEnd_Attack`
  ;[1 1 1] Collision of Sword Capsule  - Normal Attack
  (`PrimitiveComponent.SetCollisionEnabled` (`self.Capsule`) "NoCollision"))

(event `OnColStart_Skill1Attack`
  ;[1 1 1] Collision of Left hand Swrod - Skill Attack
  (`PrimitiveComponent.SetCollisionEnabled` (`self.Capsule1`) "QueryAndPhysics"))

(event `OnColEnd_Skill1Attack`
  ;[1 1 1] Collision of Left hand Swrod - Skill Attack
  (`PrimitiveComponent.SetCollisionEnabled` (`self.Capsule1`) "NoCollision"))

(fn `UserConstructionScript`)